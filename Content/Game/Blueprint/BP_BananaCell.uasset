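; BP_BananaCell is a banana actor that can be activated for collection as part of a banana quest.
; Activate runs ActivateBananaCell, which ignores already collected bananas and checks the custom game mode's state manager for an active quest.
; An inactive quest shows a French notification that the banana belongs to someone; otherwise CollectBanana is called.
; CollectBanana and HideBanana are empty stubs here.
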(event EventBeginPlay
  (|CallParentFunction)
  (bind _asbp_custom_game_mode (Utilities|Casting|CastToBP_CustomGameMode (Game|GetGameMode)))
  (Variables|Default|SetAs%20BP%20Custom%20Game%20Mode _asbp_custom_game_mode))

(event Collision|EventActorBeginOverlap
  (params (OtherActor :type Actor%20Object%20Reference))
  (|CallParentFunction OtherActor) ; This node is disabled and will not be called.\nDrag off pins to build functionality.
)

(event EventTick
  (params (DeltaSeconds :type Float%20%28single-precision%29))
  (|CallParentFunction DeltaSeconds) ; This node is disabled and will not be called.\nDrag off pins to build functionality.
)

(event EventActivate
  (params (Pawn :type BP%20Pawn%20Object%20Reference))
  (CallFunction|ActivateBananaCell))

(fn ConstructionScript
  (|CallParentFunction))

(fn ActivateBananaCell
  (bind _as_bp_custom_game_mode (Variables|Default|GetAs%20BP%20Custom%20Game%20Mode))
  (bind _as_bp_custom_game_mode_2 (Variables|Default|GetAs%20BP%20Custom%20Game%20Mode))
  (bind _bpc_gamestatemanager (Variables|/Game/Game/Blueprint/BP_CustomGameMode.BP_CustomGameMode_C|GetBPC_GameStateManager _as_bp_custom_game_mode))
  (bind _bpc_notificationmanager (Variables|/Game/Game/Blueprint/BP_CustomGameMode.BP_CustomGameMode_C|GetBPC_NotificationManager _as_bp_custom_game_mode_2))
  (Utilities|FlowControl|Sequence
    (:then_0
      (if (Variables|Default|GetIsCollect)
        (return)))
    (:then_1
      (if (and (!= _bpc_gamestatemanager 0) (not (Default|IsBananaQuestActive? _bpc_gamestatemanager)))
        (Utilities|FlowControl|Sequence
          (:then_0
            (if (!= _bpc_notificationmanager 0)
              (Default|ShowNotification _bpc_notificationmanager "Cette banane appartient a quelqu'un...")))
          (:then_1
            (return)))))
    (:then_2
      (CallFunction|CollectBanana))))

(fn CollectBanana)

(fn HideBanana)