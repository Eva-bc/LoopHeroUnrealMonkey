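; BP_Gate is a gate that swings open once enough items have been collected.
; CollectItem increments a counter and, when it reaches MaxItemsCollectable, fires OpenDoor a single time through a DoOnce.
; OpenDoor plays a timeline whose curve lerps the Door component's relative yaw to rotate it open.
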(event Custom|OpenDoor
  ;[0.15 0.15 0.15 0.5] Animation de l'ouverture porte
  (bind _door_rotation (Timeline|Open%20Door%20Animation Play)
    (:Update
      (Transformation|SetRelativeRotation (Variables|Default|GetDoor) (Math|Rotator|MakeRotator 0.0 0.0 (Math|Float|Lerp 0.0 1.2e+02 _door_rotation)) false false))))

(event Custom|Collect%20Item
  (Math|Integer|IncrementInt (Variables|Default|GetCurrentItemsCollected)
    (:%20%20
      (if (>= (Variables|Default|GetCurrentItemsCollected) (Variables|Default|GetMaxItemsCollectable))
        (Utilities|FlowControl|DoOnce false
          (:Completed
            (CallFunction|OpenDoor)))))))

(fn ConstructionScript)