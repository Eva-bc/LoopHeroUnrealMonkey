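; AI controller for the JohnnyKiki character that runs its behavior tree and feeds it targets from perception.
; On begin play it starts the tree and caches the controlled pawn.
; Perception updates set the attacking flag false unless a tagged actor is sensed.
; For sensed tagged actors, it stores the target and sets the flag by a squared-distance check against the pawn's attack range.
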(event OnTargetPerceptionUpdated(AIPerception)
  (params (Actor :type Actor%20Object%20Reference) (Stimulus :type AI%20Stimulus%20Structure))
  (bind _bsuccessfullysensed (Utilities|Struct|BreakAIStimulus Stimulus))
  (bind _targettag (Variables|Default|GetTargetTag))
  (bind _blackboard (Variables|Default|GetBlackboard))
  (bind _returnvalue (Actor|ActorHasTag Actor _targettag))
  (bind _returnvalue_2 (and _bsuccessfullysensed _returnvalue))
  (AI|Components|Blackboard|SetValueasBool _blackboard (Variables|Default|GetIsAttackingBBValue) _returnvalue_2)
  (if _returnvalue_2
    (AI|Components|Blackboard|SetValueasObject _blackboard (Variables|Default|GetTargetBBValue) Actor)
    (AI|Components|Blackboard|SetValueasBool (Variables|Default|GetBlackboard) (Variables|Default|GetIsAttackingBBValue) (<= (Class|KismetMathLibrary|VectorDistanceSquared (Transformation|GetActorLocation Actor) (Transformation|GetActorLocation (Pawn|GetControlledPawn))) (Math|Float|Power (Variables|/Game/Game/Blueprint/BP_JohnnyKiki.BP_JohnnyKiki_C|GetAttackRange (Variables|Default|GetAs%20BP%20Johnny%20Kiki)) 2.0)))))

(event EventBeginPlay
  (AI|RunBehaviorTree "/Game/Game/Blueprint/BT_JohnnyKIki.BT_JohnnyKIki")
  (bind _asbp_johnny_kiki (Utilities|Casting|CastToBP_JohnnyKiki (Pawn|GetControlledPawn)))
  (Variables|Default|SetAs%20BP%20Johnny%20Kiki _asbp_johnny_kiki))

(event EventTick
  (params (DeltaSeconds :type Float%20%28single-precision%29)))

(fn ConstructionScript)